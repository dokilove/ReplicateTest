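; BP_PS, apparently a PlayerState, holds a player's HP and UID and provides damage, alive and HP-percent functions.
; On BeginPlay it fills HP to max and has the owning BP_PC initialize its pawn.
; HP bar events named Server and Client chain into updates on BP_PC, but nothing here triggers them.
; Damage only subtracts HP and prints it, and the CurrentHP OnRep is empty.
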(event `InitPS`
  (bind _asbp_pc (cast `/Game/Blueprints/BP_PC` (`self.GetOwner`)))
  (`/Engine/EditorBlueprintResources/StandardMacros.IsValid` _asbp_pc
    (:`Is Valid`
      (`/Game/Blueprints/BP_PC.InitPawn` _asbp_pc))))

(event `InitPSServer`
  (`self.InitPS`))

(event `self.ReceiveBeginPlay`
  (`self.InitHP`)
  (bind _asbp_pc (cast `/Game/Blueprints/BP_PC` (`self.GetOwner`)))
  (`/Engine/EditorBlueprintResources/StandardMacros.IsValid` _asbp_pc
    (:`Is Valid`
      (`/Game/Blueprints/BP_PC.InitPawn` _asbp_pc))))

(event `SetHPBarPercentServer`
  (`self.SetHPBarPercentClient`))

(event `SetHPBarPercentClient`
  (`self.SetHPBarPercent`))

(event `Owner_SetUID`
  (params (UID :type Integer))
  (bind _output_get (set `self.UID` UID)))

(fn `GetHPPercent`
  (returns (Percent :type "Float (double-precision)"))
  (return (/ (`self.CurrentHP`) (`self.MaxHP`))))

(fn `InitHP`
  (set `self.CurrentHP` (`self.MaxHP`)))

(fn `IsAlive`
  (returns (IsAlive :type Boolean))
  (return (> (`self.CurrentHP`) 0.0)))

(fn `OnRep_CurrentHP`)

(fn `OnTakeDamage`
  (params (Damage :type "Float (double-precision)"))
  (set `self.CurrentHP` (- (`self.CurrentHP`) Damage))
  (`KismetSystemLibrary.PrintString` (`KismetStringLibrary.Concat_StrStr` (`KismetSystemLibrary.GetDisplayName` self) (`KismetStringLibrary.Conv_DoubleToString` (`self.CurrentHP`)) " / " (`KismetStringLibrary.Conv_DoubleToString` (`self.MaxHP`))) true true (struct :`R` 1.0 :`G` 0.042476 :`A` 1.0)))

(fn `SetHPBarPercent`
  (bind _maxhp (`self.MaxHP`))
  (bind _currenthp (`self.CurrentHP`))
  (bind _asbp_pc (cast `/Game/Blueprints/BP_PC` (`self.GetOwner`)))
  (`/Engine/EditorBlueprintResources/StandardMacros.IsValid` _asbp_pc
    (:`Is Valid`
      (`/Game/Blueprints/BP_PC.SetHPBarPercent` _asbp_pc (/ _currenthp _maxhp))
      (`/Game/Blueprints/BP_PC.SetHPBarText` _asbp_pc _currenthp _maxhp))))

(fn `UserConstructionScript`)