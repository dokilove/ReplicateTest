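; BP_GM is a game mode Blueprint that assigns an ID to each player who logs in.
; PostLogin casts the new player to BP_PC, gets its BP_PS player state, increments the PlyaerNumber counter and passes the result to OwnerSetUID.
; GameEnd only prints a debug string.
; A disconnected, authority-gated chain that would update the game state's player count and set numbered character names never runs.
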(event `self.K2_PostLogin`
  (params (NewPlayer :type "PlayerController Object Reference"))
  (bind _asbp_pc (cast `/Game/Blueprints/BP_PC` NewPlayer))
  (bind _asbp_ps (cast `/Game/Blueprints/BP_PS` (`Controller.PlayerState` _asbp_pc)))
  (bind _result (`/Engine/EditorBlueprintResources/StandardMacros.IncrementInt` (`self.PlyaerNumber`))
    (:`  `
      (`/Game/Blueprints/BP_PS.Owner_SetUID` _asbp_ps _result))))

(event `GameEnd`
  (`KismetSystemLibrary.PrintString` "GameEnd"))

(fn `UserConstructionScript`)