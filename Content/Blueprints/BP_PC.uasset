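; BP_PC is a player controller that owns the local player's HUD and displays HP for the player and two others.
; On BeginPlay, the local controller creates PlayerWidget and adds it to the viewport, while non-local controllers print a debug string.
; Setter functions push bar percentages and HP text into that widget, each guarded by IsLocalController.
; The player's own text is built from current and max HP, while the others receive ready-made text.
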(event `self.ReceiveBeginPlay`
  (if (`self.IsLocalController`)
    (bind _returnvalue (`|CreateWidget` "/Game/UI/PlayerWidget.PlayerWidget_C"))
    (set `self.PlayerWidget` _returnvalue)
    (`UserWidget.AddToViewport` _returnvalue 0)
    (else
      (`KismetSystemLibrary.PrintString` "Is Not Local"))))

(fn `SetHPBarPercent`
  (params (Percent :type "Float (double-precision)"))
  (if (`self.IsLocalController`)
    (`ProgressBar.SetPercent` (`/Game/UI/PlayerWidget.HPBarWidget` (`self.PlayerWidget`)) Percent)))

(fn `SetHPBarPercentOther1`
  (params (Percent :type "Float (double-precision)"))
  (if (`self.IsLocalController`)
    (`ProgressBar.SetPercent` (`/Game/UI/PlayerWidget.HPBarWidgetOther1` (`self.PlayerWidget`)) Percent)))

(fn `SetHPBarPercentOther2`
  (params (Percent :type "Float (double-precision)"))
  (if (`self.IsLocalController`)
    (`ProgressBar.SetPercent` (`/Game/UI/PlayerWidget.HPBarWidgetOther2` (`self.PlayerWidget`)) Percent)))

(fn `SetHPBarText`
  (params (CurrentHP :type "Float (double-precision)") (MaxHP :type "Float (double-precision)"))
  (if (`self.IsLocalController`)
    (`TextBlock.SetText` (`/Game/UI/PlayerWidget.HPTextWidget` (`self.PlayerWidget`)) (`KismetTextLibrary.Conv_StringToText` (`KismetStringLibrary.Concat_StrStr` (`KismetStringLibrary.Conv_DoubleToString` CurrentHP) " / " (`KismetStringLibrary.Conv_DoubleToString` MaxHP))))))

(fn `SetHPBarTextOther1`
  (params (HPText :type Text))
  (if (`self.IsLocalController`)
    (`TextBlock.SetText` (`/Game/UI/PlayerWidget.HPTextWidgetOther1` (`self.PlayerWidget`)) HPText)))

(fn `SetHPBarTextOther2`
  (params (HPText :type Text))
  (if (`self.IsLocalController`)
    (`TextBlock.SetText` (`/Game/UI/PlayerWidget.HPTextWidgetOther2` (`self.PlayerWidget`)) HPText)))

(fn `UserConstructionScript`)