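; BP_GS is the game state that tracks a shared respawn count and triggers game end when it runs out.
; On BeginPlay the authority sets RespawnCount to MaxRespawnCount.
; DecreaseRespawnCount decrements it and calls GameEnd on BP_GM once it reaches zero or below.
; LogUIDS prints each BP_PS UID from PlayerArray for debugging, while OnRep_PlayerCount is an empty stub.
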(event `self.ReceiveBeginPlay`
  (`self.InitRespawnCount`)
  (`KismetSystemLibrary.PrintString` (`KismetStringLibrary.Concat_StrStr` (`KismetSystemLibrary.GetDisplayName` self) "BeginPlay") true true (struct :`R` 1.0 :`B` 0.338195 :`A` 1.0) 20.0))

(event `DecreaseRespawnCount`
  (bind _respawncount (`self.RespawnCount`))
  (`/Engine/EditorBlueprintResources/StandardMacros.DecrementInt` _respawncount
    (:`  `
      (if (not (> _respawncount 0))
        (bind _asbp_gm (cast `/Game/Blueprints/BP_GM` (`GameplayStatics.GetGameMode`)))
        (`/Engine/EditorBlueprintResources/StandardMacros.IsValid` _asbp_gm
          (:`Is Valid`
            (`/Game/Blueprints/BP_GM.GameEnd` _asbp_gm)))))))

(event `LogUIDS`
  (bind _playerarray (`self.PlayerArray`))
  (for (_array_element _array_index) _playerarray
    (bind _asbp_ps (cast `/Game/Blueprints/BP_PS` _array_element))
    (`KismetSystemLibrary.PrintString` (`KismetTextLibrary.Conv_TextToString` (`|FormatText` "Length {0} : Index {1} : UID  {2}" (`KismetArrayLibrary.Array_Length` _playerarray) _array_index (`/Game/Blueprints/BP_PS.UID` _asbp_ps))) true true (struct :`R` 0.019965 :`G` 0.307292 :`A` 1.0) 120.0)))

(fn `InitRespawnCount`
  (`/Engine/EditorBlueprintResources/ActorMacros.Switch Has Authority`
    (:`Authority`
      (set `self.RespawnCount` (`self.MaxRespawnCount`)))))

(fn `OnRep_PlayerCount`)

(fn `UserConstructionScript`)